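; Player controller Blueprint that sets up game-only input and opens the pause menu.
; On BeginPlay it switches input to game-only and hides the mouse cursor.
; Pressing Escape creates a new BP_PauseUI widget, stores it and adds it to the viewport, then pauses the game and switches to game-and-UI input with the cursor shown.
; It contains no resume logic.
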(event EventBeginPlay
  (Input|SetInputModeGameOnly (Game|GetPlayerController 0) false)
  (Variables|Default|SetbShowMouseCursor false))

(event EventTick
  (params (DeltaSeconds :type Float%20%28single-precision%29)))

(event Input|ActionEvents|InputActionEscape
  (params (Key :type Key%20Structure :default "None"))
  (:Pressed
    (bind _returnvalue (UserInterface|CreateWidget "/Game/BP_PauseUI.BP_PauseUI_C"))
    (bind _output_get (Variables|Default|SetPauseMenuInstance _returnvalue))
    (UserInterface|Viewport|AddtoViewport _output_get 0)
    (Game|SetGamePaused true)
    (Input|SetInputModeGameandUI (Game|GetPlayerController 0) 0 "DoNotLock" true false)
    (Variables|Default|SetbShowMouseCursor true)))

(fn ConstructionScript)